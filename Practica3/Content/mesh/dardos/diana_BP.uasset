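; Dartboard Blueprint that catches a dart and displays points when hit.
; On a hit to the dartboard cylinder by the referenced Dardo, it attaches the dart to the board's root, keeping its world transform.
; It then sets the Puntuacion text to PuntosInt plus a fixed bonus, without writing the sum back to PuntosInt.
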(event `self.SM_DartboardDarts_Cylinder.OnComponentHit`
  (params (HitComponent :type "PrimitiveComponent Object Reference") (OtherActor :type "Actor Object Reference") (OtherComp :type "PrimitiveComponent Object Reference") (NormalImpulse :type "Vector Structure") (Hit :type "HitResult Structure (by ref)"))
  (if (== OtherActor (`self.dardo`))
    (`self.K2_AttachToComponent` (`self.dardo`) (`self.RootComponent`) "None" "KeepWorld" "KeepWorld" "KeepWorld" true)
    (`TextRenderComponent.K2_SetText` (`self.puntuacion`) (`|GenericToText` (+ (`self.puntosInt`) 10)))))

(fn `UserConstructionScript`)